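; Game manager for a day-based judging game: it serves cases, scores verdicts and runs each day's timer.
; Verdicts are checked against the current DataTable row, recorded in VerdictMass and rewarded with GameInstance money when correct, then the next case loads.
; A Tick-driven Delay counts down; timeout or the last case triggers a DoOnce-guarded fade and result screen.
; Nextday swaps case tables, resets counters and advances the pre-work row for Wednesday and Friday.
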(event Custom|NextCase
  (bind _returnvalue (Utilities|GetDataTableRow (Variables|Default|GetDayDT) (Variables|Default|GetCase))
    (:then
      (Development|PrintString (.Словаподсудимого (Utilities|Struct|BreakS_Case _returnvalue)))
      (bind _outrownames (DataTable|GetDataTableRowNames (Variables|Default|GetDayDT)))
      (if (>= (Utilities|Array|FindItem _outrownames (Variables|Default|GetCase)) 0)
        (if (Utilities|Array|IsValidIndex _outrownames (+ (Utilities|Array|FindItem _outrownames (Variables|Default|GetCase)) 1))
          (Variables|Default|SetCase (Utilities|Array|Get(acopy) _outrownames (+ (Utilities|Array|FindItem _outrownames (Variables|Default|GetCase)) 1)))
          (Math|Integer|IncrementInt (Variables|Default|GetCaseCount))
          (else
            (Math|Integer|IncrementInt (Variables|Default|GetCaseCount)
              (:%20%20
                (CallFunction|EndDay)))))))))

(event Custom|Verdict
  (if (Utilities|Enum|Equal(Enum) (Variables|Default|GetVerdict_Top) "NewEnumerator1")
    (bind _returnvalue (Utilities|GetDataTableRow (Variables|Default|GetDayDT) (Variables|Default|GetCase))
      (:then
        (if (Utilities|Enum|Equal(Enum) (Variables|Default|GetVerdict_Top) (.VerdictTop (Utilities|Struct|BreakS_Case _returnvalue)))
          (Development|PrintString "Правильно" true true "(R=0.144738,G=1.000000,B=0.184923,A=1.000000)")
          (CallFunction|GetMoney)
          (Utilities|Array|Add (Variables|Default|GetVerdictMass) true)
          (CallFunction|NextCase)
          (else
            (Development|PrintString "Не Правильно" true true "(R=1.000000,G=0.032287,B=0.623961,A=1.000000)")
            (Utilities|Array|Add (Variables|Default|GetVerdictMass) false)
            (CallFunction|NextCase)))))
    (else
      (bind _returnvalue_2 (Utilities|GetDataTableRow (Variables|Default|GetDayDT) (Variables|Default|GetCase))
        (:then
          (if (Utilities|Enum|Equal(Enum) (Variables|Default|GetVerdict_Top) (.VerdictTop (Utilities|Struct|BreakS_Case _returnvalue_2)))
            (bind _returnvalue_3 (Utilities|GetDataTableRow (Variables|Default|GetDayDT) (Variables|Default|GetCase))
              (:then
                (if (Utilities|Enum|Equal(Enum) (.VerdictBottom (Utilities|Struct|BreakS_Case _returnvalue_3)) (Variables|Default|GetVerdict_Bottom))
                  (Development|PrintString "Правильно" true true "(R=0.144738,G=1.000000,B=0.184923,A=1.000000)")
                  (CallFunction|GetMoney)
                  (Utilities|Array|Add (Variables|Default|GetVerdictMass) true)
                  (CallFunction|NextCase)
                  (else
                    (Development|PrintString "Не Правильно" true true "(R=1.000000,G=0.140562,B=0.150510,A=1.000000)")
                    (Utilities|Array|Add (Variables|Default|GetVerdictMass) false)
                    (CallFunction|NextCase)))))
            (else
              (Development|PrintString "Не Правильно" true true "(R=0.144738,G=1.000000,B=0.184923,A=1.000000)")
              (Utilities|Array|Add (Variables|Default|GetVerdictMass) false)
              (CallFunction|NextCase))))))))

(event Custom|Next%20day
  ;[0.02594 1 0.2132] Смена дня
  (bind _output_get (Variables|Default|SetCurrentDay (Utilities|Enum|ByteToEnumE_Day (+ (Variables|Default|GetCurrentDay) 1))))
  (switch Utilities|FlowControl|Switch|SwitchonE_Day _output_get
    (:NewEnumerator1
      (Variables|Default|SetCase "NewRow")
      (Variables|Default|SetDayDT "/Game/Data/Day_2.Day_2")
      (Variables|Default|SetCaseInADay 5)
      (Variables|Default|SetCaseCount 1)
      (Variables|Default|SetMinutes 10)
      (Variables|Default|SetSeconds 20))
    (:NewEnumerator2
      (Variables|Default|SetCase "NewRow")
      (Variables|Default|SetDayDT "/Game/Data/Day_3.Day_3")
      (Variables|Default|SetCaseInADay 5)
      (Variables|Default|SetCaseCount 1)
      (Variables|Default|SetMinutes 1)
      (Variables|Default|SetSeconds 20)))
  (Utilities|Array|Clear (Variables|Default|GetVerdictMass))
  (bind _outrownames (DataTable|GetDataTableRowNames "/Game/Data/DT_BeforWork.DT_BeforWork"))
  (if (>= (Utilities|Array|FindItem _outrownames (Variables|Default|GetBeforDayName)) 0)
    (if (Utilities|Array|IsValidIndex _outrownames (+ (Utilities|Array|FindItem _outrownames (Variables|Default|GetBeforDayName)) 1))
      (Variables|Default|SetBeforDayName (Utilities|Array|Get(acopy) _outrownames (+ (Utilities|Array|FindItem _outrownames (Variables|Default|GetBeforDayName)) 1)))
      (CallFunction|RestartTimer))))

(event Custom|Test0
  (if (Utilities|Enum|Equal(Enum) (Variables|Default|GetVerdict_Top) "NewEnumerator1")
    (bind _returnvalue (Utilities|GetDataTableRow (Variables|Default|GetDayDT) (Variables|Default|GetCase))
      (:then
        (if (Utilities|Enum|Equal(Enum) (Variables|Default|GetVerdict_Top) (.VerdictTop (Utilities|Struct|BreakS_Case _returnvalue)))
          (Development|PrintString "Правильно" true true "(R=0.144738,G=1.000000,B=0.184923,A=1.000000)")
          (CallFunction|GetMoney)
          (Utilities|Array|Add (Variables|Default|GetVerdictMass) true)
          (CallFunction|NextCase)
          (else
            (Development|PrintString "Не Правильно" true true "(R=1.000000,G=0.032287,B=0.623961,A=1.000000)")
            (Utilities|Array|Add (Variables|Default|GetVerdictMass) false)
            (CallFunction|NextCase)))))
    (else
      (bind _returnvalue_2 (Utilities|GetDataTableRow (Variables|Default|GetDayDT) (Variables|Default|GetCase))
        (:then
          (if (Utilities|Enum|Equal(Enum) (Variables|Default|GetVerdict_Top) (.VerdictTop (Utilities|Struct|BreakS_Case _returnvalue_2)))
            (bind _returnvalue_3 (Utilities|GetDataTableRow (Variables|Default|GetDayDT) (Variables|Default|GetCase))
              (:then
                (if (Utilities|Enum|Equal(Enum) (.VerdictBottom (Utilities|Struct|BreakS_Case _returnvalue_3)) (Variables|Default|GetVerdict_Bottom))
                  (Development|PrintString "Правильно" true true "(R=0.144738,G=1.000000,B=0.184923,A=1.000000)")
                  (CallFunction|GetMoney)
                  (Utilities|Array|Add (Variables|Default|GetVerdictMass) true)
                  (CallFunction|NextCase)
                  (else
                    (Development|PrintString "Не Правильно" true true "(R=1.000000,G=0.140562,B=0.150510,A=1.000000)")
                    (Utilities|Array|Add (Variables|Default|GetVerdictMass) false)
                    (CallFunction|NextCase)))))
            (else
              (Development|PrintString "Не Правильно" true true "(R=0.144738,G=1.000000,B=0.184923,A=1.000000)")
              (Utilities|Array|Add (Variables|Default|GetVerdictMass) false)
              (CallFunction|NextCase))))))))

(event Custom|TimerEvent
  ;[1 1 1] Таймер
  (Utilities|FlowControl|Delay 1.0)
  (if (<= (Variables|Default|GetSeconds) 0)
    (if (<= (Variables|Default|GetMinutes) 0)
      (CallFunction|EndDay)
      (else
        (Variables|Default|SetSeconds 59)
        (Math|Integer|DecrementInt (Variables|Default|GetMinutes))))
    (else
      (Math|Integer|DecrementInt (Variables|Default|GetSeconds)))))

(event Custom|Start/StopTimerEvent
  ;[1 1 1] Таймер
  (Variables|Default|SetStart/StopTimer true))

(event Custom|EndDay
  (Utilities|FlowControl|DoOnce false
    (:Completed
      (Variables|Default|SetStart/StopTimer false)
      (bind _returnvalue (UserInterface|CreateWidget "/Game/UI/UI_FadeIn.UI_FadeIn_C"))
      (UserInterface|Viewport|AddtoViewport _returnvalue 0)
      (Utilities|FlowControl|Delay 1.5)
      (bind _returnvalue_2 (UserInterface|CreateWidget "/Game/UI/Courtroom/UI_Result.UI_Result_C"))
      (UserInterface|Viewport|AddtoViewport _returnvalue_2 0))))

(event Custom|Restart%20timer
  (Utilities|FlowControl|DoOnce false) ; enters at Reset
)

(event Custom|GetMoney
  (bind _asbp_gi_money (Utilities|Casting|CastToBP_GI_Money (Game|GetGameInstance)))
  (bind _output_get (Variables|/Game/BP/BP_GI_Money.BP_GI_Money_C|SetMoneyInst _asbp_gi_money (+ (Variables|/Game/BP/BP_GI_Money.BP_GI_Money_C|GetMoneyInst _asbp_gi_money) 100)))
  (Development|PrintString (Utilities|String|Append "Сейчас денег: " (Utilities|String|ToString(Integer) _output_get))))

(event Custom|Sound%20click
  (Utilities|ClickSoundMacro))

(event EventTick
  (params (DeltaSeconds :type Float%20%28single-precision%29))
  ;[1 1 1] Таймер
  (if (Variables|Default|GetStart/StopTimer)
    (CallFunction|TimerEvent)))

(event EventBeginPlay
  ;[1 1 1] Разные вещи
  (Variables|/Script/Engine.PlayerController|SetbShowMouseCursor (Game|GetPlayerController 0) true))

(fn ConstructionScript)