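; BP_PC, apparently the player controller, handles UI hotkeys and test shortcuts.
; It creates an exit widget at BeginPlay and toggles it on screen through the Exit event, Escape or the 2 key.
; Other keys show a timed fade-out widget or call BP_GM game mode functions for the verdict, money and a test routine.
; A further key opens the titles map.
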(event Custom|Exit
  (bind _newvar (Variables|Default|GetNewVar))
  (if (Variables|Default|GetExit_UI)
    (Variables|Default|SetExit_UI false)
    (Widget|RemovefromParent _newvar)
    (else
      (Variables|Default|SetExit_UI true)
      (UserInterface|Viewport|AddtoViewport _newvar 0))))

(event EventBeginPlay
  (bind _returnvalue (UserInterface|CreateWidget "/Game/UI/Courtroom/UI_Exit.UI_Exit_C"))
  (Variables|Default|SetNewVar _returnvalue))

(event EventTick
  (params (DeltaSeconds :type Float%20%28single-precision%29)))

(event Input|KeyboardEvents|1
  (params (Key :type Key%20Structure :default "None"))
  (:Pressed
    (bind _returnvalue (UserInterface|CreateWidget "/Game/UI/UI_FadeOut.UI_FadeOut_C"))
    (UserInterface|Viewport|AddtoViewport _returnvalue 0)
    (Utilities|FlowControl|Delay 1.5)
    (Widget|RemovefromParent _returnvalue)))

(event Input|KeyboardEvents|Escape
  (params (Key :type Key%20Structure :default "None"))
  (bind _newvar (Variables|Default|GetNewVar))
  (:Pressed
    (if (Variables|Default|GetExit_UI)
      (Variables|Default|SetExit_UI false)
      (Widget|RemovefromParent _newvar)
      (else
        (Variables|Default|SetExit_UI true)
        (UserInterface|Viewport|AddtoViewport _newvar 0)))))

(event Input|KeyboardEvents|2
  (params (Key :type Key%20Structure :default "None"))
  (bind _newvar (Variables|Default|GetNewVar))
  (:Pressed
    (if (Variables|Default|GetExit_UI)
      (Variables|Default|SetExit_UI false)
      (Widget|RemovefromParent _newvar)
      (else
        (Variables|Default|SetExit_UI true)
        (UserInterface|Viewport|AddtoViewport _newvar 0)))))

(event Input|KeyboardEvents|3
  (params (Key :type Key%20Structure :default "None"))
  (:Pressed
    (bind _asbp_gm (Utilities|Casting|CastToBP_GM (Game|GetGameMode)))
    (Default|Verdict _asbp_gm)))

(event Input|KeyboardEvents|0
  (params (Key :type Key%20Structure :default "None"))
  ;[1 1 1] Тестовая часть
  (:Pressed
    (bind _asbp_gm (Utilities|Casting|CastToBP_GM (Game|GetGameMode)))
    (Default|Test0 _asbp_gm)))

(event Input|KeyboardEvents|Z
  (params (Key :type Key%20Structure :default "None"))
  (:Pressed
    (bind _asbp_gm (Utilities|Casting|CastToBP_GM (Game|GetGameMode)))
    (Default|GetMoney _asbp_gm)))

(event Input|KeyboardEvents|X
  (params (Key :type Key%20Structure :default "None"))
  (:Pressed
    (Game|OpenLevel(byName) "TitlesMap")))

(fn ConstructionScript)